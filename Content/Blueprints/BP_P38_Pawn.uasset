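; BP_P38_Pawn is a player-flown P-38 plane pawn that moves forward constantly and fires rockets.
; Tick drives forward movement input, while Pitch and Roll axes rotate the actor locally, scaled by delta time and RotateSpeed.
; Fire spawns a Rocket at the plane's transform.
; BeginPlay registers the Left and Right components with BPRotateSceneComponent for rotation; a local RotatePropeller function is defined but not called here.
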(event `self.ReceiveBeginPlay`
  (`KismetArrayLibrary.Array_Add` (`/Game/Blueprints/BP_RotateSceneComponent.SceneComponenets` (`self.BP_RotateSceneComponent`)) (`self.Left`))
  (`KismetArrayLibrary.Array_Add` (`/Game/Blueprints/BP_RotateSceneComponent.SceneComponenets` (`self.BP_RotateSceneComponent`)) (`self.Right`)))

(event `self.ReceiveTick`
  (params (DeltaSeconds :type "Float (single-precision)"))
  (`self.AddMovementInput` (`self.GetActorForwardVector`)))

(event `InputAxis|Pitch`
  (params (AxisValue :type "Float (single-precision)"))
  (`self.K2_AddActorLocalRotation` (`KismetMathLibrary.MakeRotator` 0.0 (* AxisValue (`GameplayStatics.GetWorldDeltaSeconds`) (`self.RotateSpeed`)))))

(event `InputAxis|Roll`
  (params (AxisValue :type "Float (single-precision)"))
  (`self.K2_AddActorLocalRotation` (`KismetMathLibrary.MakeRotator` (* AxisValue (`GameplayStatics.GetWorldDeltaSeconds`) (`self.RotateSpeed`)))))

(event `InputAction|Fire`
  (params (Key :type "Key Structure"))
  (:`Pressed`
    (`|SpawnActorFromClass` "/Game/Blueprints/Rocket.Rocket_C" (`self.GetTransform`) "AlwaysSpawn" "MultiplyWithRoot" null null)))

(fn `RotatePropeller`
  (params (Where :type "SceneComponent Object Reference"))
  (`SceneComponent.K2_AddLocalRotation` Where (`KismetMathLibrary.MakeRotator` (* (`GameplayStatics.GetWorldDeltaSeconds`) (`self.Speed`))) false false))

(fn `UserConstructionScript`)